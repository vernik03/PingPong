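; Player controller for a networked Pong game that owns the player's HUD widget and relays match events to it.
; On BeginPlay it creates WBP_HUD and adds it to the viewport, only where it lacks authority.
; StartGameUI waits briefly, then starts the HUD's game display on that same non-authority side.
; ChangeScoreUI passes both players' scores to the HUD without an authority check.
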(event EventBeginPlay
  (Networking|SwitchHasAuthority
    (:Remote
      (bind _returnvalue (UserInterface|CreateWidget "/Game/UI/WBP_HUD.WBP_HUD_C" self))
      (bind _output_get (Variables|Default|SetHUD _returnvalue))
      (UserInterface|Viewport|AddtoViewport _output_get 0))))

(event EventStartGameUI
  (Utilities|FlowControl|Delay 0.2)
  (Networking|SwitchHasAuthority
    (:Remote
      (Default|StartGame (Variables|Default|GetHUD)))))

(event EventChangeScoreUI
  (params (Player1Score :type Integer) (Player2Score :type Integer))
  (Default|SetScore (Variables|Default|GetHUD) Player1Score Player2Score))

(fn ConstructionScript)